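; Player pawn Blueprint that turns Enhanced Input actions into movement, look and sprint state calls.
; On possession by a player controller, it registers its input mapping context.
; Move axes are cached and sent together to StateMove, with releases forwarded only while the two axes differ.
; Turn input drives StateLook, look-up reaches it only at zero, and jog override starts sprint on trigger and ends it on cancel.
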(event `EnhancedInput|/Game/Locomotion/Inputs/IA_MoveRight`
  (params (ActionValue :type "Float (double-precision)") (ElapsedSeconds :type "Float (double-precision)") (TriggeredSeconds :type "Float (double-precision)") (InputAction :type "InputAction Object Reference" :default "/Game/Locomotion/Inputs/IA_MoveRight.IA_MoveRight"))
  ;[0.2622 0.6244 1] Inputs
  (:`Triggered`
    (bind _output_get (set `self.MoveX` ActionValue))
    (`self.StateMove` _output_get (stale `EnhancedInput|/Game/Locomotion/Inputs/IA_MoveForward` _output_get) :!label _label))
  (:`Completed`
    (set `self.MoveX` 0.0)
    (if (not (== (`self.MoveX`) (`self.MoveY`))) :!label _label_2
      (goto _label))))

(event `EnhancedInput|/Game/Locomotion/Inputs/IA_MoveForward`
  (params (ActionValue :type "Float (double-precision)") (ElapsedSeconds :type "Float (double-precision)") (TriggeredSeconds :type "Float (double-precision)") (InputAction :type "InputAction Object Reference" :default "/Game/Locomotion/Inputs/IA_MoveForward.IA_MoveForward"))
  ;[0.2622 0.6244 1] Inputs
  (:`Triggered`
    (bind _output_get (set `self.MoveY` ActionValue))
    (goto _label))
  (:`Completed`
    (set `self.MoveY` 0.0)
    (goto _label_2)))

(event `EnhancedInput|/Game/Locomotion/Inputs/IA_LookTurn`
  (params (ActionValue :type "Float (double-precision)") (ElapsedSeconds :type "Float (double-precision)") (TriggeredSeconds :type "Float (double-precision)") (InputAction :type "InputAction Object Reference" :default "/Game/Locomotion/Inputs/IA_LookTurn.IA_LookTurn"))
  ;[0.2622 0.6244 1] Inputs
  (:`Triggered`
    (`self.StateLook` ActionValue (stale `EnhancedInput|/Game/Locomotion/Inputs/IA_LookUp` ActionValue) :!label _label_3)))

(event `EnhancedInput|/Game/Locomotion/Inputs/IA_LookUp`
  (params (ActionValue :type "Float (double-precision)") (ElapsedSeconds :type "Float (double-precision)") (TriggeredSeconds :type "Float (double-precision)") (InputAction :type "InputAction Object Reference" :default "/Game/Locomotion/Inputs/IA_LookUp.IA_LookUp"))
  ;[0.2622 0.6244 1] Inputs
  (:`Triggered`
    (if (== (stale `EnhancedInput|/Game/Locomotion/Inputs/IA_LookTurn` ActionValue) 0.0)
      (goto _label_3))))

(event `EnhancedInput|/Game/Locomotion/Inputs/IA_JogOverride`
  (params (ActionValue :type Boolean) (ElapsedSeconds :type "Float (double-precision)") (TriggeredSeconds :type "Float (double-precision)") (InputAction :type "InputAction Object Reference" :default "/Game/Locomotion/Inputs/IA_JogOverride.IA_JogOverride"))
  ;[0.2622 0.6244 1] Inputs
  (:`Triggered`
    (`self.StateSprintStart`))
  (:`Canceled`
    (`self.StateSprintEnd`)))

(event `self.ReceiveBeginPlay`)

(event `self.ReceivePossessed`
  (params (NewController :type "Controller Object Reference"))
  (bind _asplayer_controller (cast `PlayerController` NewController))
  (`EnhancedInputSubsystemInterface.AddMappingContext` (pcsubsystem `EnhancedInputLocalPlayerSubsystem` _asplayer_controller) "/Game/Locomotion/Inputs/InputMappingContext.InputMappingContext" 0 (struct)))

(fn `UserConstructionScript`)